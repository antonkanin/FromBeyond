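; Player character with axis-driven movement and look, timed hazard damage, and quest note pickup.
; It creates the player and blood-effect HUDs, and overlapping a BP_DeathZone starts a looping Damage timer that is paused on exit.
; Damage broadcasts health and effect updates, opening BusStopLevel when health runs out.
; Interact line-traces from the camera to store and print notes; Tick draws a debug facing line.
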(event Collision|EventActorEndOverlap
  (params (OtherActor :type Actor%20Object%20Reference))
  ;[1 1 1] Character Health Management
  (Utilities|Casting|CastToBP_DeathZone OtherActor)
  (Utilities|Time|PauseTimerbyHandle (Variables|Default|GetTimerHandle))
  (Default|CallEnableHealthEffect false))

(event EventTick
  (params (DeltaSeconds :type Float%20%28single-precision%29))
  (bind _returnvalue (Transformation|GetActorTransform))
  (bind _location (Math|Transform|BreakTransform _returnvalue))
  (Rendering|Debug|DrawDebugLine :LineStart _location :LineEnd (+ _location (* (Transformation|GetActorForwardVector (Pawn|GetController)) 1e+02)) :Thickness 1.0))

(event Collision|EventActorBeginOverlap
  (params (OtherActor :type Actor%20Object%20Reference))
  ;[1 1 1] Character Health Management
  (Utilities|Casting|CastToBP_DeathZone OtherActor)
  (bind _returnvalue (Utilities|Time|SetTimerbyFunctionName 0 "Damage" 0.5 true))
  (Variables|Default|SetTimerHandle _returnvalue))

(event EventBeginPlay
  (bind _returnvalue (UserInterface|CreateWidget "/Game/Blueprints/UI/PlayerHUD.PlayerHUD_C"))
  (UserInterface|Viewport|AddtoViewport _returnvalue 0)
  (bind _returnvalue_2 (UserInterface|CreateWidget "/Game/Blueprints/UI/BloodEffectHUD.BloodEffectHUD_C"))
  (bind _output_get (Variables|Default|SetBloodEffectReference _returnvalue_2))
  (UserInterface|Viewport|AddtoViewport _output_get 0))

(event Input|ActionEvents|InputActionInteract
  (params (Key :type Key%20Structure))
  (bind _camera (Variables|Default|GetCamera))
  (bind _returnvalue (Transformation|GetWorldLocation _camera))
  ;[1 1 1] Picking up quest notes
  (:Pressed
    (bind _outhit (Collision|LineTraceByChannel _returnvalue (+ _returnvalue (* (Math|Vector|GetForwardVector _camera) 1e+02)) "TraceTypeQuery1" false 0 "Persistent"))
    (bind _asbp_quest_note (Utilities|Casting|CastToBP_QuestNote (.HitActor (Collision|BreakHitResult _outhit))))
    (Utilities|Array|Add (Variables|Default|GetQuestNotes) _asbp_quest_note)
    (Development|PrintString (Utilities|String|Append "You've found a note: " (Utilities|String|ToString(Text) (Variables|/Game/Blueprints/BP_QuestNote.BP_QuestNote_C|GetNoteText _asbp_quest_note))))))

(event Input|AxisEvents|InputAxisMoveForward
  (params (AxisValue :type Float%20%28single-precision%29))
  ;[1 1 1] Character Basic Movement
  (Pawn|Input|AddMovementInput (Math|Vector|GetForwardVector (Variables|Character|GetMesh)) AxisValue false))

(event Input|AxisEvents|InputAxisMoveRight
  (params (AxisValue :type Float%20%28single-precision%29))
  ;[1 1 1] Character Basic Movement
  (Pawn|Input|AddMovementInput (Math|Vector|GetRightVector (Variables|Character|GetMesh)) AxisValue false))

(event Input|AxisEvents|InputAxisLookUp
  (params (AxisValue :type Float%20%28single-precision%29))
  ;[1 1 1] Character Basic Movement
  (Pawn|Input|AddControllerPitchInput AxisValue))

(event Input|AxisEvents|InputAxisTurnRight
  (params (AxisValue :type Float%20%28single-precision%29))
  ;[1 1 1] Character Basic Movement
  (Pawn|Input|AddControllerYawInput AxisValue))

(fn ConstructionScript)

(fn Damage
  (bind _output_get (Variables|Default|SetCurrentHealth (- (Variables|Default|GetCurrentHealth) 1e+01)))
  (Default|CallUpdateHealth _output_get)
  (Default|CallEnableHealthEffect true)
  ;[1 1 1] If the player's health is less then 0 we just restart the level
  (if (<= _output_get 0.0)
    (Game|OpenLevel(byName) "BusStopLevel")))